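; BP_RealPlayer is a player Character Blueprint that handles basic looking, movement and jumping.
; Turn Right and Look Up axis inputs drive controller yaw and pitch, and the Jump action triggers a jump.
; Every Tick, the Vertical and Horizontal values form a normalized direction, rotated by the full control rotation and fed into AddMovementInput for view-relative movement.
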(event `InputAxis|Turn Right`
  (params (AxisValue :type "Float (single-precision)"))
  ;[1 1 1] Comment
  (`self.AddControllerYawInput` AxisValue))

(event `InputAxis|Look Up`
  (params (AxisValue :type "Float (single-precision)"))
  ;[1 1 1] Comment
  (`self.AddControllerPitchInput` AxisValue))

(event `self.ReceiveTick`
  (params (DeltaSeconds :type "Float (single-precision)"))
  ;[1 1 1] Comment
  (`self.AddMovementInput` (`KismetMathLibrary.TransformDirection` (`KismetMathLibrary.MakeTransform` (0.0 0.0 0.0) (`self.GetControlRotation`)) (`KismetMathLibrary.Normal` (`KismetMathLibrary.MakeVector` (`self.GetInputAxisValue`) (`self.GetInputAxisValue`))))))

(event `InputAction|Jump`
  (params (Key :type "Key Structure"))
  ;[1 1 1] Comment
  (:`Pressed`
    (`self.Jump`)))

(fn `UserConstructionScript`)